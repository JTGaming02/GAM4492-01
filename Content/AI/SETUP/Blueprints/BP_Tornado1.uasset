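; BP_Tornado1 is a tornado AI enemy that damages EBS buildings it touches and flags itself as a melee enemy on BeginPlay.
; Capsule overlap applies damage once and sets a looping timer on the same function, which takes inputs a by-name timer cannot supply.
; The timer is never cleared on the live path.
; A separate durability-based damage function is uncalled here, and older delay, perception and destroy nodes are disconnected.
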(event `self.ReceiveBeginPlay`
  ;[1 1 1] Specify enemy type
  (`parent.ReceiveBeginPlay`)
  (`self.IMeleeEnemy`))

(event `self.Capsule.OnComponentBeginOverlap`
  (params (OverlappedComponent :type "PrimitiveComponent Object Reference") (OtherActor :type "Actor Object Reference") (OtherComp :type "PrimitiveComponent Object Reference") (OtherBodyIndex :type Integer) (bFromSweep :type Boolean) (SweepResult :type "HitResult Structure (by ref)"))
  ;[1 1 1] Tornado Damage
  (bind _asbp_ebs_building_base_object (cast `/Game/Building/Blueprints/BuildingObjects/Base/BP_EBS_Building_BaseObject` OtherActor))
  (`self.ApplyTornadoDamage_0` _asbp_ebs_building_base_object 50.0)
  (`KismetSystemLibrary.K2_SetTimer` null "ApplyTornadoDamage_0" 0.5 true))

(fn `ApplyDamageToBuildings`
  (params (TargetBuilding :type "Actor Object Reference") (DamageAmount :type "Float (double-precision)" :default -200.0))
  (bind _asdurability (cast `/Game/Building/Blueprints/Interfaces/Durability` TargetBuilding))
  (`/Game/Building/Blueprints/BuildingObjects/Base/BP_EBS_Building_BaseObject.ChangeDurability_BPI` (cast `/Game/Building/Blueprints/BuildingObjects/Base/BP_EBS_Building_BaseObject` _asdurability :!pure true) "NewEnumerator1" DamageAmount))

(fn `ApplyTornadoDamage_0`
  (params (TargetBuilding :type "/Game/Building/Blueprints/BuildingObjects/Base/BP_EBS_Building_BaseObject Object Reference") (DamageAmount :type "Float (double-precision)" :default 1.0))
  (`KismetSystemLibrary.PrintString` "9")
  (`GameplayStatics.ApplyDamage` TargetBuilding DamageAmount)
  (`KismetSystemLibrary.PrintString` "Its workin"))

(fn `UserConstructionScript`
  (`parent.UserConstructionScript`))