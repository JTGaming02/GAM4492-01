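; Blueprint function library of shared helpers for enemy AI, covering the player, buildings and BP_Enemy.
; Player helpers wrap a BuilderCharacter cast for target, death and name-indexed stats; others toggle enemy damage, rotation, task-change flags and stencil outlines.
; Building helpers scan all EBS building actors for the closest or first, and report hit sphere, facing and destruction.
; CastSkill reads a DataTable and deducts caster cost, but its skill-spawn branch is disconnected.
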(fn `allowDamage`
  (params (Enemy :type "Actor Object Reference") (Allow :type Boolean))
  (bind _asbp_enemy (cast `/Game/AI/SETUP/Blueprints/AI/BP_Enemy` Enemy)
    (:`then`
      (set `/Game/AI/SETUP/Blueprints/AI/BP_Enemy.DamageAvaliable` Allow _asbp_enemy))
    (:`CastFailed`
      (`KismetSystemLibrary.PrintString` null "AI is not inherited from BP_Enemy (Call from allowDamage)" true true (struct :`R` 1.0 :`A` 1.0)))))

(fn `allowRotation`
  (params (Enemy :type "Actor Object Reference") (Allow :type Boolean))
  (bind _asbp_enemy (cast `/Game/AI/SETUP/Blueprints/AI/BP_Enemy` Enemy)
    (:`then`
      (set `/Game/AI/SETUP/Blueprints/AI/BP_Enemy.RotationBlocked` (not Allow) _asbp_enemy))
    (:`CastFailed`
      (`KismetSystemLibrary.PrintString` null "AI is not inherited from BP_Enemy (Call from allowRotation)" true true (struct :`R` 1.0 :`A` 1.0)))))

(fn `allowTaskChange`
  (params (Enemy :type "Actor Object Reference") (Allow :type Boolean))
  (bind _asbp_enemy (cast `/Game/AI/SETUP/Blueprints/AI/BP_Enemy` Enemy)
    (:`then`
      (set `/Game/AI/SETUP/Blueprints/AI/BP_Enemy.RangeAttackInProgress` (not Allow) _asbp_enemy))
    (:`CastFailed`
      (`KismetSystemLibrary.PrintString` null "AI is not inherited from BP_Enemy (Call from allowTaskChange)" true true (struct :`R` 1.0 :`A` 1.0)))))

(fn `CastSkill`
  (params (SkillID :type Name) (Owner :type "Actor Object Reference") (__WorldContext :type "Object Object Reference"))
  (returns (Success :type Boolean) (Cooldown :type "Float (double-precision)"))
  (locals (SkillUsed :type Boolean :default true) (SkillCooldown :type "Float (double-precision)") (ID :type Name) (SkillOwner :type "Actor Object Reference") (SkillStats :type "/Game/AI/SETUP/Blueprints/Skills/Requirements Structure" :default (struct :`CostStat` "Mana")))
  (bind (_skillbp _name _description _coststat _cost) (break `/Game/AI/SETUP/Blueprints/Skills/Requirements` (`local.SkillStats`)))
  (bind (_skillbp_2 _name_2 _description_2 _coststat_2 _cost_2) (break `/Game/AI/SETUP/Blueprints/Skills/Requirements` (`local.SkillStats`)))
  (bind _value (`self.GetPlayersState` _coststat_2))
  ;[1 1 1] Initialize local variables
  (set `local.ID` SkillID)
  (set `local.SkillOwner` Owner)
  (bind _returnvalue (`|GetDataTableRow` "/Game/AI/SETUP/Blueprints/Skills/SkillsTable.SkillsTable" (`local.ID`))
    (:`then`
      (set `local.SkillStats` _returnvalue)
      ;[1 1 1] Who is caster?
      (bind _asbp_enemy (cast `/Game/AI/SETUP/Blueprints/AI/BP_Enemy` (`local.SkillOwner`))
        (:`then`
          (bind _statcurrent (`/Game/AI/SETUP/Blueprints/AI/BP_Enemy.StatCurrent` _asbp_enemy))
          (bind _output (`|GetArrayItem` _statcurrent 1))
          ;[1 1 1] Used by enemy
          (if (> _cost _output)
            ;[1 1 1] Failed
            (set `local.SkillUsed` false :!label _label)
            (return (`local.SkillUsed`) (`local.SkillCooldown`))
            (else
              (`KismetArrayLibrary.Array_Set` _statcurrent 1 (- _output _cost)))))
        (:`CastFailed`
          ;[1 1 1] Used by player
          (if (> _cost_2 _value)
            (goto _label)
            (else
              (`self.SetPlayersState` (`.CostStat_17_EF0EA2DB40133811FAFDB28B4153E603` (break `/Game/AI/SETUP/Blueprints/Skills/Requirements` (`local.SkillStats`))) (- _value _cost_2)))))))
    (:`RowNotFound`
      (goto _label))))

(fn `Distance Between Actor And Closest Building`
  (params (Actor :type "Actor Object Reference"))
  (returns (Distance :type "Float (double-precision)") (ClosestBuilding :type "/Game/Building/Blueprints/BuildingObjects/Base/BP_EBS_Building_BaseObject Object Reference"))
  (locals (ClosestDistance :type "Float (double-precision)" :default 9999.0) (TornadoREF :type "/Game/AI/SETUP/Blueprints/BP_Tornado Object Reference") (MinDistance :type "Float (double-precision)") (EnemyAiREF :type "/Game/AI/SETUP/Blueprints/AI/BP_Enemy Object Reference") (CloseBuilding :type "/Game/Building/Blueprints/BuildingObjects/Base/BP_EBS_Building_BaseObject Object Reference"))
  ;[1 1 1] To Find Closest building and its distance
  (bind _outactors (`GameplayStatics.GetAllActorsOfClass` null "/Game/Building/Blueprints/BuildingObjects/Base/BP_EBS_Building_BaseObject.BP_EBS_Building_BaseObject_C"))
  (if (== (`KismetArrayLibrary.Array_Length` _outactors) 0)
    (return 0.0 null)
    (else
      (bind _output_get (set `local.CloseBuilding` (`|GetArrayItem` _outactors)))
      (set `local.ClosestDistance` (`KismetMathLibrary.Vector_Distance` (`Actor.K2_GetActorLocation` _output_get) (`Actor.K2_GetActorLocation` Actor)))
      (for (_array_element _array_index) _outactors
        (bind _returnvalue (`KismetMathLibrary.Vector_Distance` (`Actor.K2_GetActorLocation` _array_element) (`Actor.K2_GetActorLocation` Actor)))
        (if (< _returnvalue (`local.ClosestDistance`))
          (set `local.CloseBuilding` (`|GetArrayItem` _outactors _array_index))
          (set `local.ClosestDistance` _returnvalue)))
      (return (`local.ClosestDistance`) (`local.CloseBuilding`)))))

(fn `DistanceBetweenActorAndPlayer`
  (params (Actor :type "Actor Object Reference"))
  (returns (Distance :type "Float (double-precision)"))
  (return (`KismetMathLibrary.VSize` (- (`Actor.K2_GetActorLocation` Actor) (`Actor.K2_GetActorLocation` (`GameplayStatics.GetPlayerCharacter` null))))))

(fn `GetBuilding`
  (returns (BuildingRef :type "/Game/Building/Blueprints/BuildingObjects/Base/BP_EBS_Building_BaseObject Object Reference"))
  (bind _outactors (`GameplayStatics.GetAllActorsOfClass` null "/Game/Building/Blueprints/BuildingObjects/Base/BP_EBS_Building_BaseObject.BP_EBS_Building_BaseObject_C"))
  (for _array_element _outactors
    (return _array_element)))

(fn `GetBuildingHitBox`
  (params (Building :type "/Game/Building/Blueprints/BuildingObjects/Base/BP_EBS_Building_BaseObject Object Reference"))
  (returns (HitBox :type "StaticMeshComponent Object Reference"))
  (`/Engine/EditorBlueprintResources/StandardMacros.IsValid` Building
    (:`Is Valid`
      (return (`/Game/Building/Blueprints/BuildingObjects/Base/BP_EBS_Building_BaseObject.HitSphere` Building)))
    (:`Is Not Valid`
      (`KismetSystemLibrary.PrintString` null "HBF/Invalid player reference (Call from getPlayersTarget)" true true (struct :`R` 1.0 :`A` 1.0))
      (return null))))

(fn `GetBuildingLocation`
  (params (Building :type "/Game/Building/Blueprints/BuildingObjects/Base/BP_EBS_Building_BaseObject Object Reference"))
  (returns (Location :type "Vector Structure"))
  (return (`Actor.K2_GetActorLocation` Building)))

(fn `GetPlayer`
  (returns (BuildingOBJRef :type "/Game/Building/Blueprints/Character/BuilderCharacter Object Reference"))
  (bind _asbuilder_character (cast `/Game/Building/Blueprints/Character/BuilderCharacter` (`GameplayStatics.GetPlayerCharacter` null))
    (:`then`
      (return _asbuilder_character))
    (:`CastFailed`
      (`KismetSystemLibrary.PrintString` null "Player is not inherited from CharacterBaseClass (Call from getPlayer)" true true (struct :`R` 1.0 :`A` 1.0))
      (return null))))

(fn `GetPlayersHitBox`
  (returns (HitBox :type "StaticMeshComponent Object Reference"))
  (bind _buildingobjref (`self.GetPlayer` null))
  (`/Engine/EditorBlueprintResources/StandardMacros.IsValid` _buildingobjref
    (:`Is Valid`
      (return (`/Game/Building/Blueprints/Character/BuilderCharacter.HitSphere` _buildingobjref)))
    (:`Is Not Valid`
      (`KismetSystemLibrary.PrintString` null "Invalid player reference (Call from getPlayersTarget)" true true (struct :`R` 1.0 :`A` 1.0))
      (return null))))

(fn `GetPlayersLocation`
  (returns (Location :type "Vector Structure"))
  (return (`Actor.K2_GetActorLocation` (`GameplayStatics.GetPlayerCharacter` null))))

(fn `GetPlayersState`
  (params (StatName :type Name))
  (returns (Value :type "Float (double-precision)"))
  (locals (StatValue :type "Float (double-precision)"))
  (bind _buildingobjref (`self.GetPlayer` null))
  (bind _returnvalue (`KismetArrayLibrary.Array_Find` (`/Game/Building/Blueprints/Character/BuilderCharacter.StatName` _buildingobjref) StatName))
  (`/Engine/EditorBlueprintResources/StandardMacros.IsValid` _buildingobjref
    (:`Is Valid`
      (if (== _returnvalue -1)
        (`KismetSystemLibrary.PrintString` null "Can't find stat" true true (struct :`R` 1.0 :`A` 1.0))
        (else
          ;[1 1 1] get value by index
          (set `local.StatValue` (`|GetArrayItem` (`/Game/Building/Blueprints/Character/BuilderCharacter.StatCurrent` _buildingobjref) _returnvalue))))
      (return (`local.StatValue`)))
    (:`Is Not Valid`
      (`KismetSystemLibrary.PrintString` null "Invalid player reference (Call from getPlayersStat)" true true (struct :`R` 1.0 :`A` 1.0))
      (return 0.0))))

(fn `GetPlayersStateMax`
  (params (StatName :type Name))
  (returns (Value :type "Float (double-precision)"))
  (locals (StatValue :type "Float (double-precision)"))
  (bind _buildingobjref (`self.GetPlayer` null))
  (bind _returnvalue (`KismetArrayLibrary.Array_Find` (`/Game/Building/Blueprints/Character/BuilderCharacter.StatName` _buildingobjref) StatName))
  (`/Engine/EditorBlueprintResources/StandardMacros.IsValid` _buildingobjref
    (:`Is Valid`
      (if (== _returnvalue -1)
        (`KismetSystemLibrary.PrintString` null "Can't find stat maximum" true true (struct :`R` 1.0 :`A` 1.0))
        (else
          ;[1 1 1] get value by index
          (set `local.StatValue` (`|GetArrayItem` (`/Game/Building/Blueprints/Character/BuilderCharacter.StatMax` _buildingobjref) _returnvalue))))
      (return (`local.StatValue`)))
    (:`Is Not Valid`
      (`KismetSystemLibrary.PrintString` null "Invalid player reference (Call from getPlayersStatMax)" true true (struct :`R` 1.0 :`A` 1.0))
      (return 0.0))))

(fn `GetPlayersStateMin`
  (params (StatName :type Name))
  (returns (Value :type "Float (double-precision)"))
  (locals (StatValue :type "Float (double-precision)"))
  (bind _buildingobjref (`self.GetPlayer` null))
  (bind _returnvalue (`KismetArrayLibrary.Array_Find` (`/Game/Building/Blueprints/Character/BuilderCharacter.StatName` _buildingobjref) StatName))
  (`/Engine/EditorBlueprintResources/StandardMacros.IsValid` _buildingobjref
    (:`Is Valid`
      (if (== _returnvalue -1)
        (`KismetSystemLibrary.PrintString` null "Can't find stat minimum" true true (struct :`R` 1.0 :`A` 1.0))
        (else
          ;[1 1 1] get value by index
          (set `local.StatValue` (`|GetArrayItem` (`/Game/Building/Blueprints/Character/BuilderCharacter.StatMin` _buildingobjref) _returnvalue))))
      (return (`local.StatValue`)))
    (:`Is Not Valid`
      (`KismetSystemLibrary.PrintString` null "Invalid player reference (Call from getPlayersStatMin)" true true (struct :`R` 1.0 :`A` 1.0))
      (return 0.0))))

(fn `GetPlayersTarget`
  (returns (TargetActor :type "Actor Object Reference"))
  (bind _buildingobjref (`self.GetPlayer` null))
  (`/Engine/EditorBlueprintResources/StandardMacros.IsValid` _buildingobjref
    (:`Is Valid`
      (return (`/Game/Building/Blueprints/Character/BuilderCharacter.TargetActor` _buildingobjref)))
    (:`Is Not Valid`
      (`KismetSystemLibrary.PrintString` null "Invalid player reference (Call from getPlayersTarget)" true true (struct :`R` 1.0 :`A` 1.0))
      (return null))))

(fn `GetPlayersTargetWidget`
  (returns (WidgetRef :type "/Game/AI/SETUP/UI/WB_TargetWidget Object Reference"))
  (bind _buildingobjref (`self.GetPlayer` null))
  (`/Engine/EditorBlueprintResources/StandardMacros.IsValid` _buildingobjref
    (:`Is Valid`
      (return (`/Game/Building/Blueprints/Character/BuilderCharacter.TargetHUDWidget` _buildingobjref)))
    (:`Is Not Valid`
      (`KismetSystemLibrary.PrintString` null "Invalid player reference (Call from getPlayersTargetWidget)" true true (struct :`R` 1.0 :`A` 1.0))
      (return null))))

(fn `GetRotationToBuilding`
  (params (Actor :type "Actor Object Reference") (Building :type "/Game/Building/Blueprints/BuildingObjects/Base/BP_EBS_Building_BaseObject Object Reference"))
  (returns (Rot :type "Rotator Structure"))
  (return (`KismetMathLibrary.MakeRotator` 0.0 0.0 (.yaw (`KismetMathLibrary.FindLookAtRotation` (`Actor.K2_GetActorLocation` Actor) (`Actor.K2_GetActorLocation` Building))))))

(fn `GetRotationToPlayer`
  (params (Actor :type "Actor Object Reference"))
  (returns (Rot :type "Rotator Structure"))
  (return (`KismetMathLibrary.MakeRotator` 0.0 0.0 (.yaw (`KismetMathLibrary.FindLookAtRotation` (`Actor.K2_GetActorLocation` Actor) (`Actor.K2_GetActorLocation` (`GameplayStatics.GetPlayerCharacter` null)))))))

(fn `IsBuildingDestroyed?`
  (params (Building :type "/Game/Building/Blueprints/BuildingObjects/Base/BP_EBS_Building_BaseObject Object Reference"))
  (returns (IsDestroyed :type Boolean))
  (`/Engine/EditorBlueprintResources/StandardMacros.IsValid` Building
    (:`Is Valid`
      (bind _currentvalue (`/Game/Building/Blueprints/BuildingObjects/Base/BP_EBS_Building_BaseObject.GetDurability_BPI` Building))
      (return (<= _currentvalue 0.0)))
    (:`Is Not Valid`
      (`KismetSystemLibrary.PrintString` null "Invalid Building  reference (Call from isBuilding destroyed?)" true true (struct :`R` 1.0 :`A` 1.0))
      (return false))))

(fn `IsPlayerDead?`
  (returns (IsDead :type Boolean))
  (bind _buildingobjref (`self.GetPlayer` null))
  (`/Engine/EditorBlueprintResources/StandardMacros.IsValid` _buildingobjref
    (:`Is Valid`
      (return (`/Game/Building/Blueprints/Character/BuilderCharacter.IsDead` _buildingobjref)))
    (:`Is Not Valid`
      (`KismetSystemLibrary.PrintString` null "Invalid player reference (Call from isPlayerDead?)" true true (struct :`R` 1.0 :`A` 1.0))
      (return false))))

(fn `SetOutline`
  (params (ComponentForOutline :type "PrimitiveComponent Object Reference") (`On/Off` :type Boolean))
  (locals (Material :type "MaterialInstanceDynamic Object Reference") (Led :type Boolean) (Component :type "PrimitiveComponent Object Reference"))
  ;[1 1 1] Initialize local variables
  (set `local.Component` ComponentForOutline)
  (set `local.Led` `On/Off`)
  ;[1 1 1] Set outline if component is not equal to null
  (if (!= (`local.Component`) null)
    ;[1 1 1] You can add custom outline for each actor type here. Just connect logic to CastFailed
    (bind _asbp_enemy (cast `/Game/AI/SETUP/Blueprints/AI/BP_Enemy` (`ActorComponent.GetOwner` (`local.Component`))))
    ;[1 1 1] Works with Void Lantern Outliner. Disconnect StencilValue section, if your outline material is not working with stencils
    (`PrimitiveComponent.SetRenderCustomDepth` (`local.Component`) (`local.Led`))
    (`PrimitiveComponent.SetCustomDepthStencilValue` (`local.Component`) (`/Game/AI/SETUP/Blueprints/AI/BP_Enemy.OutlineColor` _asbp_enemy))))

(fn `SetPlayersState`
  (params (StatName :type Name) (Value :type "Float (double-precision)"))
  (bind _buildingobjref (`self.GetPlayer` null))
  (bind _returnvalue (`KismetArrayLibrary.Array_Find` (`/Game/Building/Blueprints/Character/BuilderCharacter.StatName` _buildingobjref) StatName))
  (`/Engine/EditorBlueprintResources/StandardMacros.IsValid` _buildingobjref
    (:`Is Valid`
      (if (== _returnvalue -1)
        (`KismetSystemLibrary.PrintString` null "Can't set stat - stat not found")
        (else
          (`KismetArrayLibrary.Array_Set` (`/Game/Building/Blueprints/Character/BuilderCharacter.StatCurrent` _buildingobjref) _returnvalue (`KismetMathLibrary.FClamp` Value (`|GetArrayItem` (`/Game/Building/Blueprints/Character/BuilderCharacter.StatMin` _buildingobjref) _returnvalue) (`|GetArrayItem` (`/Game/Building/Blueprints/Character/BuilderCharacter.StatMax` _buildingobjref) _returnvalue))))))
    (:`Is Not Valid`
      (`KismetSystemLibrary.PrintString` null "Invalid player reference (Call from setPlayersState)" true true (struct :`R` 1.0 :`A` 1.0)))))

(fn `SetPlayersTarget`
  (params (Actor :type "Actor Object Reference"))
  (bind _buildingobjref (`self.GetPlayer` null))
  (`/Engine/EditorBlueprintResources/StandardMacros.IsValid` _buildingobjref
    (:`Is Valid`
      (set `/Game/Building/Blueprints/Character/BuilderCharacter.TargetActor` Actor _buildingobjref))
    (:`Is Not Valid`
      (`KismetSystemLibrary.PrintString` null "Invalid player reference (Call from setPlayersTarget)" true true (struct :`R` 1.0 :`A` 1.0)))))