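; Player character for a survival game with inventory, switchable hatchet, pickaxe and mallet stances, camera toggle and pause menu.
; Looping timers drain hunger and thirst into damage once empty, and zero health shows a respawn screen and reloads the level.
; BeginPlay also schedules timed tornado round spawners at the player's location, with Round4 scheduled twice and Round5 never.
; Tick updates climb and vault key prompts from ClimbingBP.
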(event `self.ReceiveBeginPlay`
  ;[1 1 1] Begin Play event
  (`/Game/NEW/NEW-UI/BP/AC_Inventory_component.Iintiate` (`self.AC_Inventory_component`) self)
  (`parent.ReceiveBeginPlay`)
  (bind _foundwidgets (`WidgetBlueprintLibrary.GetAllWidgetsOfClass` "/Game/Movement/HUD/HUD_Widget.HUD_Widget_C"))
  (set `self.HUD` (`|GetArrayItem` _foundwidgets))
  ;;[1 0.191 0.9392] Display stats
  (bind _returnvalue (`|CreateWidget` "/Game/NEW/NEW-UI/WB/HUD-Gamble.HUD-Gamble_C"))
  (bind _output_get (set `self.G-hud` _returnvalue))
  (`UserWidget.AddToViewport` _output_get 0)
  (`self.DrainThirst`)
  (`self.Hunger_Drain`)
  ;[1 1 1] Spawn/Despawn Tornado For Each Round After Specific Time
  (`|ExecutionSequence`
    (:`then_0`
      (`KismetSystemLibrary.K2_SetTimer` null "SpawnTornado" 5.0)
      (`KismetSystemLibrary.K2_SetTimer` null "SpawnTornadoRound1" 125.0)
      (`KismetSystemLibrary.K2_SetTimer` null "SpawnTornadoRound2" 210.0)
      (`KismetSystemLibrary.K2_SetTimer` null "SpawnTornadoRound3" 290.0)
      (`KismetSystemLibrary.K2_SetTimer` null "SpawnTornadoRound4" 380.0)
      (`KismetSystemLibrary.K2_SetTimer` null "SpawnTornadoRound4" 500.0))))

(event `EnhancedInput|/Game/Movement/Data/Inputs/IA_ChangeCamera`
  (params (ActionValue :type Boolean) (ElapsedSeconds :type "Float (double-precision)") (TriggeredSeconds :type "Float (double-precision)") (InputAction :type "InputAction Object Reference" :default "/Game/Movement/Data/Inputs/IA_ChangeCamera.IA_ChangeCamera"))
  ;[1 1 1] ChangeCamera
  (:`Triggered`
    (switch `/Game/Movement/Data/Enum/E_CameraType` (`/Game/Movement/CharacterComponents/M_BaseComponent_BP.CameraType` (`self.BaseComponent_BP`))
      (:`NewEnumerator0`
        (`ActorComponent.Deactivate` (`self.FPC`))
        (`ActorComponent.Activate` (`self.TPC`) true))
      (:`NewEnumerator1`
        (`ActorComponent.Deactivate` (`self.TPC`))
        (`ActorComponent.Activate` (`self.FPC`) true)))))

(event `EnhancedInput|/Game/Movement/Data/Inputs/IA_Menu`
  (params (ActionValue :type Boolean) (ElapsedSeconds :type "Float (double-precision)") (TriggeredSeconds :type "Float (double-precision)") (InputAction :type "InputAction Object Reference" :default "/Game/Movement/Data/Inputs/IA_Menu.IA_Menu"))
  ;[1 1 1] HUD
  (:`Triggered`
    (bind _menu (`self.Menu`)
      (:`then`
        (`Widget.RemoveFromParent` _menu)
        (set `self.Menu` null)
        (set `PlayerController.bShowMouseCursor` false (`GameplayStatics.GetPlayerController` 0))
        (`GameplayStatics.SetGamePaused` false))
      (:`else`
        (bind _returnvalue (`|CreateWidget` "/Game/Movement/HUD/Menu_Widget.Menu_Widget_C"))
        (bind _output_get (set `self.Menu` _returnvalue))
        (`UserWidget.AddToViewport` _output_get 0)
        (set `PlayerController.bShowMouseCursor` true (`GameplayStatics.GetPlayerController` 0))
        (`GameplayStatics.SetGamePaused` true)))))

(event `self.ReceiveTick`
  (params (DeltaSeconds :type "Float (single-precision)"))
  (bind _climbing_bp (`self.Climbing_BP`))
  (bind _climbing_bp_2 (`self.Climbing_BP`))
  (bind _canstartvaultingmode (`/Game/Movement/CharacterComponents/SystemComponents/Climbing_BP.CanStartVaultingMode` (`self.Climbing_BP`)))
  ;[1 1 1] Tick event
  (`parent.ReceiveTick` DeltaSeconds)
  ;;[1 1 1] Screen Prompts (HUD)
  (if (and (`/Game/Movement/CharacterComponents/SystemComponents/Climbing_BP.CanStartClimbing` _climbing_bp) (not (`/Game/Movement/CharacterComponents/SystemComponents/Climbing_BP.ManualClimbingPerformanceMode` _climbing_bp)))
    (`self.ClimbingPrompt`
      (:`then`
        _)
      (:`else`
        (bind _returnvalue (`|CreateWidget` "/Game/Movement/HUD/KeyBinds_Widget.KeyBinds_Widget_C" null "E" "Climb"))
        (bind _output_get (set `self.ClimbingPrompt` _returnvalue))
        (`VerticalBox.AddChildToVerticalBox` (`/Game/Movement/HUD/HUD_Widget.MidScreenPrompt` (`self.HUD`)) _output_get)))
    (else
      (bind _climbingprompt (`self.ClimbingPrompt`)
        (:`then`
          (`PanelWidget.RemoveChild` (`/Game/Movement/HUD/HUD_Widget.MidScreenPrompt` (`self.HUD`)) _climbingprompt)
          (set `self.ClimbingPrompt` null))
        (:`else`
          _))))
  (if (and (`/Game/Movement/CharacterComponents/SystemComponents/Climbing_BP.CanStartVaulting` _climbing_bp_2) (not (`/Game/Movement/CharacterComponents/SystemComponents/Climbing_BP.ManualClimbingPerformanceMode` _climbing_bp_2)))
    (`self.ClimbDownPrompt`
      (:`then`)
      (:`else`
        (bind _returnvalue_2 (`|CreateWidget` "/Game/Movement/HUD/KeyBinds_Widget.KeyBinds_Widget_C" null (select `/Game/Movement/Data/Enum/E_VaultMode` _canstartvaultingmode :`NewEnumerator0` "E" :`NewEnumerator1` "X" :`NewEnumerator2` "E" :`NewEnumerator3` "X" :!type "Text") (select `/Game/Movement/Data/Enum/E_VaultMode` _canstartvaultingmode :`NewEnumerator0` "Climb Up" :`NewEnumerator1` "Climb Down" :`NewEnumerator2` "Vault" :`NewEnumerator3` "DropDown" :!type "Text")))
        (bind _output_get_2 (set `self.ClimbDownPrompt` _returnvalue_2))
        (`VerticalBox.AddChildToVerticalBox` (`/Game/Movement/HUD/HUD_Widget.MidScreenPrompt` (`self.HUD`)) _output_get_2)))
    (else
      (bind _climbdownprompt (`self.ClimbDownPrompt`)
        (:`then`
          (`PanelWidget.RemoveChild` (`/Game/Movement/HUD/HUD_Widget.MidScreenPrompt` (`self.HUD`)) _climbdownprompt)
          (set `self.ClimbDownPrompt` null))
        (:`else`)))))

(event `Key|One`
  (params (Key :type "Key Structure"))
  ;[1 1 1] Change interaction stance inputs
  (:`Pressed`
    (if (not (`self.IsPlayingRootMotion`))
      (`self.ChangeInteractionStance (Server)` "NewEnumerator1"))))

(event `self.ReceiveAnyDamage`
  (params (Damage :type "Float (single-precision)") (DamageType :type "DamageType Object Reference") (InstigatedBy :type "Controller Object Reference") (DamageCauser :type "Actor Object Reference"))
  ;[1 1 1] AI STUFF
  ;;[1 1 1] Taking damage from enemy
  ;;[1 0.2611 0.7589] Test Health-Shanice
  (bind _output_get (set `self.Health` (- (`self.Health`) Damage)))
  (`/Game/NEW/NEW-UI/WB/Health-Bar.SetHealth` (`/Game/NEW/NEW-UI/WB/HUD-Gamble.Health-Bar_146` (`self.G-HUD`)) (`self.Health`))
  (if (<= _output_get 0.0)
    ;;[1 1 1] Respawn Screen
    (bind _returnvalue (`|CreateWidget` "/Game/NEW/NEW-UI/WB/Respawn-Screen.Respawn-Screen_C"))
    (`UserWidget.AddToViewport` _returnvalue 0)
    (`KismetSystemLibrary.Delay` 1.0)
    (bind _returnvalue_2 (`GameplayStatics.GetCurrentLevelName` true))
    (`GameplayStatics.OpenLevel` (`KismetStringLibrary.Conv_StringToName` _returnvalue_2))))

(event `Key|Two`
  (params (Key :type "Key Structure"))
  ;[1 1 1] Change interaction stance inputs
  (:`Pressed`
    (if (not (`self.IsPlayingRootMotion`))
      (`self.ChangeInteractionStance (Server)` "NewEnumerator2"))))

(event `Key|Three`
  (params (Key :type "Key Structure"))
  ;[1 1 1] Change interaction stance inputs
  (:`Pressed`
    (if (not (`self.IsPlayingRootMotion`))
      (`self.ChangeInteractionStance (Server)` "NewEnumerator3"))))

(event `CustomEvent`
  ;[1 1 1] AI STUFF
  (`|ExecutionSequence`
    (:`then_0`
      ;;[1 1 1] Initialize variables
      (`self.Initialization`))))

(event `Key|I`
  (params (Key :type "Key Structure"))
  (bind _ac_inventory_component (`self.AC_Inventory_component`))
  ;[1 1 1] AI STUFF
  ;;[1 0.2396 0.7606] inputs for pickups and inventory
  (:`Pressed`
    (`/Engine/EditorBlueprintResources/StandardMacros.FlipFlop`
      (:`A`
        (`/Game/NEW/NEW-UI/BP/AC_Inventory_component.F_ShowInventory` _ac_inventory_component))
      (:`B`
        (`/Game/NEW/NEW-UI/BP/AC_Inventory_component.F_hideInventory` _ac_inventory_component)))))

(event `Key|F`
  (params (Key :type "Key Structure"))
  ;[1 1 1] AI STUFF
  ;;[1 0.2396 0.7606] inputs for pickups and inventory
  (:`Pressed`
    (`/Game/NEW/NEW-UI/BP/AC_Inventory_component.F_Trytopickup` (`self.AC_Inventory_component`))))

(event `self.InteractionComponent.OnInteractionStanceChanged`
  (params (NewInteractionStance :type "/Game/Building/Blueprints/Enumerations/InteractionType Enum" :default "NewEnumerator0") (PrevInteractionStance :type "/Game/Building/Blueprints/Enumerations/InteractionType Enum" :default "NewEnumerator0"))
  ;[1 1 1] Character interaction events
  (set `self.InteractionStance` NewInteractionStance))

(event `ChangeInteractionStance (Server)`
  (params (NewInteractionStance :type "/Game/Building/Blueprints/Enumerations/InteractionType Enum" :default "NewEnumerator0"))
  ;[1 1 1] Character interaction events
  (`/Game/Building/Blueprints/Components/InteractionComponent.ChangeInteractionStance` (`self.InteractionComponent`) NewInteractionStance))

(event `self.InteractionComponent.OnInteractionNotify`
  (params (Character :type "Character Object Reference") (InteractionActor :type "Actor Object Reference") (NotifyName :type Name))
  ;[1 1 1] Character interaction events
  (switch `name` NotifyName
    (:`PlayToolActAnimation`
      (`SkeletalMeshComponent.PlayAnimation` (`self.ToolMesh`) (select `/Game/Building/Blueprints/Enumerations/InteractionType` (`self.InteractionStance`) :`NewEnumerator1` "/Game/Building/Mannequin/Animations/A_Tool_Hatchet_Act.A_Tool_Hatchet_Act" :`NewEnumerator2` "/Game/Building/Mannequin/Animations/A_Tool_Pickaxe_Act.A_Tool_Pickaxe_Act" :!type "AnimationAsset Object Reference") false))))

(event `Hunger_Drain`
  ;[1 0.3581 0.8043] Hunger Drain Function
  (`KismetSystemLibrary.K2_SetTimer` null "Drain_Hunger" 2.5 true 10.0))

(event `DrainThirst`
  ;[1 0.4078 0.9083] drain thirst Function
  (`KismetSystemLibrary.K2_SetTimer` null "Drain_thirst-1" 2.5 true 10.0))

(fn `DeSpawnTornado`
  (params (Actor :type "Actor Object Reference"))
  (`KismetSystemLibrary.PrintString` "DE1" true true (struct :`R` 0.080484 :`G` 0.082743 :`B` 1.0 :`A` 1.0) 5.0)
  (for _array_element (`self.Enemy in Pack`)
    (`KismetSystemLibrary.PrintString` (`KismetSystemLibrary.GetDisplayName` _array_element) true true (struct :`G` 0.928206 :`B` 1.0 :`A` 1.0) 30.0)
    (bind _asbp_enemy (cast `/Game/AI/SETUP/Blueprints/AI/BP_Enemy` _array_element))
    (`KismetSystemLibrary.PrintString` "DE3" true true (struct :`R` 0.080484 :`G` 0.082743 :`B` 1.0 :`A` 1.0) 5.0)
    (`/Game/AI/SETUP/Blueprints/AI/BP_Enemy.OnEnemyDied` _asbp_enemy)))

(fn `Drain_Hunger`
  (bind _returnvalue (/ (`self.Hunger`) (`self.Max Hunger`)))
  (`/Engine/EditorBlueprintResources/StandardMacros.DecrementFloat` (`self.Hunger`)
    (:`  `
      (`/Game/NEW/NEW-UI/WB/Hunger-1.Set percent` (`/Game/NEW/NEW-UI/WB/HUD-Gamble.Hunger_Bar` (`self.G-HUD`)) _returnvalue)
      (if (<= _returnvalue 0.0)
        (`GameplayStatics.ApplyDamage` self 0.5)))))

(fn `Drain_thirst-1`
  (bind _returnvalue (/ (`self.Thirst`) (`self.Max Thirst`)))
  (`/Engine/EditorBlueprintResources/StandardMacros.DecrementFloat` (`self.Thirst`)
    (:`  `
      (`/Game/NEW/NEW-UI/WB/Thirst-1.Set percent` (`/Game/NEW/NEW-UI/WB/HUD-Gamble.Thirst_Bar` (`self.G-HUD`)) _returnvalue)
      (if (<= _returnvalue 0.0)
        (`GameplayStatics.ApplyDamage` self 0.5)
        (return)))))

(fn `Initialization`
  (`|ExecutionSequence`
    (:`then_0`
      ;[1 1 1] Parameters initialization
      (`/Game/AI/SETUP/Blueprints/Utility/BFL_UtilitiesLibrary.SetPlayersState` "Health" (`/Game/AI/SETUP/Blueprints/Utility/BFL_UtilitiesLibrary.GetPlayersStateMax` "Health"))
      (`/Game/AI/SETUP/Blueprints/Utility/BFL_UtilitiesLibrary.SetPlayersState` "Energy" (`/Game/AI/SETUP/Blueprints/Utility/BFL_UtilitiesLibrary.GetPlayersStateMax` "Energy")))
    (:`then_1`
      ;[1 1 1] Creating TargetWidgen and PlayerBarWidget
      (bind _returnvalue (`|CreateWidget` "/Game/AI/SETUP/UI/WB_PlayerBarWidget.WB_PlayerBarWidget_C"))
      (bind _output_get (set `/Game/Building/Blueprints/Character/BuilderCharacter.PlayerBarWidget` _returnvalue (`/Game/AI/SETUP/Blueprints/Utility/BFL_UtilitiesLibrary.GetPlayer`)))
      (`UserWidget.AddToViewport` _output_get 0))
    (:`then_2`
      (bind _returnvalue_2 (`|CreateWidget` "/Game/AI/SETUP/UI/WB_TargetWidget.WB_TargetWidget_C"))
      (bind _output_get_2 (set `/Game/Building/Blueprints/Character/BuilderCharacter.TargetHUDWidget` _returnvalue_2 (`/Game/AI/SETUP/Blueprints/Utility/BFL_UtilitiesLibrary.GetPlayer`)))
      (`UserWidget.AddToViewport` _output_get_2 0))))

(fn `OnPlayerDied`
  (`GameplayStatics.OpenLevelBySoftObjectPtr` "/Game/JonZ/Levels/HeagMainMenu.HeagMainMenu")
  (set `self.IsDead` true)
  (`self.DisableInput` (`GameplayStatics.GetPlayerCharacter` 0) (`GameplayStatics.GetPlayerController` 0))
  (`MovementComponent.StopMovementImmediately` (`self.CharacterMovement`)))

(fn `OnRep_InteractionStance`
  (`SkinnedMeshComponent.SetSkinnedAssetAndUpdate` (`self.ToolMesh`) (select `/Game/Building/Blueprints/Enumerations/InteractionType` (`self.InteractionStance`) :`NewEnumerator1` "/Game/Building/Mannequin/Mesh/SK_Tool_Hatchet_001.SK_Tool_Hatchet_001" :`NewEnumerator2` "/Game/Building/Mannequin/Mesh/SK_Tool_Pickaxe_001.SK_Tool_Pickaxe_001" :`NewEnumerator3` "/Game/Building/Mannequin/Mesh/SK_Tool_Mallet.SK_Tool_Mallet" :!type "SkeletalMesh Object Reference") true))

(fn `SpawnTornado`
  (`|SpawnActorFromClass` "/Game/AI/SETUP/Blueprints/AI/BP_Spawner.BP_Spawner_C" (`KismetMathLibrary.MakeTransform` (`self.K2_GetActorLocation`)) "Undefined" "MultiplyWithRoot" null null))

(fn `SpawnTornadoRound1`
  (`|SpawnActorFromClass` "/Game/AI/SETUP/Blueprints/AI/BP_SpawnerRound1.BP_SpawnerRound1_C" (`KismetMathLibrary.MakeTransform` (`self.K2_GetActorLocation`)) "Undefined" "MultiplyWithRoot" null null))

(fn `SpawnTornadoRound2`
  (`|SpawnActorFromClass` "/Game/AI/SETUP/Blueprints/AI/BP_SpawnerRound2.BP_SpawnerRound2_C" (`KismetMathLibrary.MakeTransform` (`self.K2_GetActorLocation`)) "Undefined" "MultiplyWithRoot" null null))

(fn `SpawnTornadoRound3`
  (`|SpawnActorFromClass` "/Game/AI/SETUP/Blueprints/AI/BP_SpawnerRound3.BP_SpawnerRound3_C" (`KismetMathLibrary.MakeTransform` (`self.K2_GetActorLocation`)) "Undefined" "MultiplyWithRoot" null null))

(fn `SpawnTornadoRound4`
  (`|SpawnActorFromClass` "/Game/AI/SETUP/Blueprints/AI/BP_SpawnerRound4.BP_SpawnerRound4_C" (`KismetMathLibrary.MakeTransform` (`self.K2_GetActorLocation`)) "Undefined" "MultiplyWithRoot" null null))

(fn `SpawnTornadoRound5`
  (`|SpawnActorFromClass` "/Game/AI/SETUP/Blueprints/AI/BP_SpawnerRound5.BP_SpawnerRound5_C" (`KismetMathLibrary.MakeTransform` (`self.K2_GetActorLocation`)) "Undefined" "MultiplyWithRoot" null null))

(fn `SwitchWeapon`)

(fn `UserConstructionScript`)