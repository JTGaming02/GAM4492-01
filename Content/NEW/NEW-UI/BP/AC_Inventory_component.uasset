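; Inventory component that stores picked-up items as classes and manages the inventory and interaction prompt widgets.
; Pickup adds the item class, plays a local or replicated sound and destroys the actor through a server event.
; Dropping spawns the class at a randomly offset point ahead of the owner, while using only removes it.
; Inventory changes refresh the UI by closing and recreating the widget, with mouse input toggled unless a controller is used.
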(event `Spawn_Item01`
  (params (Class :type "Actor Class Reference") (`Spawn Transform` :type "Transform Structure"))
  (`|SpawnActorFromClass` Class `Spawn Transform` "AlwaysSpawn" "MultiplyWithRoot" null null))

(event `Sever_PlaySound`
  (params (Sound :type "SoundBase Object Reference") (Location :type "Vector Structure"))
  (`self.MC_Playsound` Sound Location))

(event `MC_Playsound`
  (params (Sound :type "SoundBase Object Reference") (Location :type "Vector Structure"))
  (`GameplayStatics.PlaySoundAtLocation` Sound Location (struct) 1.0 1.0 0.0 null null null null))

(event `Client_Spawnitem`
  (params (Itemtospawn :type "/Game/NEW/NEW-UI/BP/Master_Item Class Reference") (`Spawn Transform` :type "Transform Structure"))
  (`self.Spawn_Item01` Itemtospawn `Spawn Transform`))

(event `/Game/NEW/NEW-UI/BP/Inventory_Interface.F_Spawnitem`
  (params (Itemtospawn :type "/Game/NEW/NEW-UI/BP/Master_Item Class Reference") (`Spawn Transform` :type "Transform Structure"))
  (`self.Client_Spawnitem` Itemtospawn `Spawn Transform`))

(event `Server_DestroyActor`
  (params (`Item To pickup` :type "Actor Object Reference"))
  (`Actor.K2_DestroyActor` `Item To pickup`))

(event `Iintiate`
  (params (`owning actor` :type "Actor Object Reference"))
  (set `self.owning actor` `owning actor`))

(event `Initiate`
  (params (`owning actor` :type "Actor Object Reference"))
  (set `self.owning actor` `owning actor`))

(event `SetInteractVisible`
  (params (Condition :type Boolean))
  (bind _myinventory (`self.Myinventory`))
  (if Condition
    (bind _returnvalue (`|CreateWidget` "/Game/NEW/NEW-UI/WB/WB_Interaction.WB_Interaction_C"))
    (bind _output_get (set `self.InteractionHud` _returnvalue))
    (`/Engine/EditorBlueprintResources/StandardMacros.IsValid` _output_get
      (:`Is Valid`
        (`UserWidget.AddToViewport` _output_get 0)))
    (else
      (`/Engine/EditorBlueprintResources/StandardMacros.IsValid` _myinventory
        (:`Is Valid`
          (`Widget.RemoveFromParent` _myinventory))))))

(fn `F_addtoinventory`
  (params (`New item` :type "/Game/NEW/NEW-UI/BP/Master_Item Object Reference"))
  (bind _returnvalue (`SceneComponent.K2_GetComponentLocation` (`/Game/NEW/NEW-UI/BP/Master_Item.StaticMesh` `New item`)))
  (`KismetArrayLibrary.Array_Add` (`self.Inventory`) (`GameplayStatics.GetObjectClass` `New item`))
  (`/Engine/EditorBlueprintResources/StandardMacros.IsValid` (`self.Myinventory`)
    (:`Is Valid`
      (`self.F_hideInventory`)
      (`self.F_ShowInventory`))
    (:`Is Not Valid`
      _))
  (if (`self.Replicate-sound?`)
    (`/Engine/EditorBlueprintResources/ActorComponentMacros.Switch Has Authority`
      (:`Authority`
        (`self.MC_Playsound` "/Game/NEW/NEW-UI/Sounds/Item-Pickup.Item-Pickup" _returnvalue))
      (:`Remote`
        (`self.Sever_PlaySound` "/Game/NEW/NEW-UI/Sounds/Item-Pickup.Item-Pickup" _returnvalue)))
    (else
      (`GameplayStatics.PlaySound2D` "/Game/NEW/NEW-UI/Sounds/Item-Pickup.Item-Pickup" 1.0 1.0 0.0 null null))))

(fn `F_Dropitem`
  (params (Itemtospawn :type "/Game/NEW/NEW-UI/BP/Master_Item Class Reference"))
  (locals (`Drop Postion` :type "Transform Structure"))
  (bind _returnvalue (`self.GetOwner`))
  (bind _inventory (`self.Inventory`))
  (set `local.Drop Postion` (`KismetMathLibrary.Conv_VectorToTransform` (+ (+ (`Actor.K2_GetActorLocation` _returnvalue) (* (`KismetMathLibrary.GetForwardVector` (`Actor.K2_GetActorRotation` _returnvalue)) (`self.Item Drop distance`))) (`KismetMathLibrary.MakeVector` (`KismetMathLibrary.RandomFloatInRange` -75.0 75.0) (`KismetMathLibrary.RandomFloatInRange` -75.0 75.0)))))
  (`self.Spawn_Item01` Itemtospawn (`local.Drop Postion`))
  (`KismetArrayLibrary.Array_Remove` _inventory (`KismetArrayLibrary.Array_Find` _inventory Itemtospawn))
  (`self.F_hideInventory`)
  (`self.F_ShowInventory`))

(fn `F_Hideinteraction`
  (`/Engine/EditorBlueprintResources/StandardMacros.IsValid` (`self.InteractionHud`)
    (:`Is Valid`
      (`Widget.RemoveFromParent` (`self.InteractionHud`)))))

(fn `F_hideInventory`
  (bind _returnvalue (`GameplayStatics.GetPlayerController` 0))
  (`/Engine/EditorBlueprintResources/StandardMacros.IsValid` (`self.Myinventory`)
    (:`Is Valid`
      (`Widget.RemoveFromParent` (`self.Myinventory`))
      (set `self.Inventoryopen` false)
      (if (not (`self.controller?`))
        (`WidgetBlueprintLibrary.SetInputMode_GameOnly` _returnvalue)
        (set `PlayerController.bShowMouseCursor` false _returnvalue)))))

(fn `F_Showinteraction`
  (bind _returnvalue (`|CreateWidget` "/Game/NEW/NEW-UI/WB/WB_Interaction.WB_Interaction_C"))
  (bind _output_get (set `self.InteractionHud` _returnvalue))
  (`/Engine/EditorBlueprintResources/StandardMacros.IsValid` _output_get
    (:`Is Valid`
      (`UserWidget.AddToViewport` _output_get 0))))

(fn `F_ShowInventory`
  (bind _returnvalue (`GameplayStatics.GetPlayerController` 0))
  (bind _returnvalue_2 (`GameplayStatics.GetPlayerController` 0))
  (if (and (not (`self.Inventoryopen`)) (`Controller.IsLocalPlayerController` _returnvalue_2))
    (bind _returnvalue_3 (`|CreateWidget` "/Game/NEW/NEW-UI/WB/WB_Inventory_Gamble.WB_Inventory_Gamble_C" _returnvalue_2))
    (set `self.Inventoryopen` true)
    (bind _output_get (set `self.Myinventory` _returnvalue_3))
    (`UserWidget.AddToViewport` _output_get 0)
    (`/Game/NEW/NEW-UI/WB/WB_Inventory_Gamble.F_Update` _returnvalue_3 (`self.Inventory`))
    (if (not (`self.controller?`))
      (`WidgetBlueprintLibrary.SetInputMode_GameAndUIEx` _returnvalue (`self.Myinventory`) "LockInFullscreen" false)
      (set `PlayerController.bShowMouseCursor` true _returnvalue))))

(fn `F_Trytopickup`
  (bind _itemtopickup (`self.Itemtopickup`))
  (if (> (`KismetArrayLibrary.Array_Length` (`self.overlapping items`)) 0)
    (`self.F_addtoinventory` _itemtopickup)
    (`KismetArrayLibrary.Array_RemoveItem` (`self.overlapping items`) _itemtopickup)
    (`self.Server_DestroyActor` (`self.Itemtopickup`))))

(fn `F_Useitem_`
  (params (Itemtospawn :type "/Game/NEW/NEW-UI/BP/Master_Item Class Reference"))
  (locals (`Drop Postion` :type "Transform Structure"))
  (bind _inventory (`self.Inventory`))
  (`KismetArrayLibrary.Array_Remove` _inventory (`KismetArrayLibrary.Array_Find` _inventory Itemtospawn))
  (`self.F_hideInventory`)
  (`self.F_ShowInventory`))